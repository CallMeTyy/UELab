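; Target spawner actor that places targets around itself for the player to hit and tracks the score.
; A looping timer spawns a Target at a random horizontal offset while the spawned count is under its cap, yawed toward the player by a look-at on the spawner's height.
; Each target receives a reference to the spawner, whose HitTarget function increments the hit count and sends it to the ScoreBoard.
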(event Custom|SpawnTarget
  (bind _returnvalue (Math|Random|RandomFloatinRange -1e+03 1e+03))
  (bind _returnvalue_2 (Math|Random|RandomFloatinRange -2e+03 2e+03))
  (bind _returnvalue_3 (Transformation|GetActorLocation))
  (bind _player (Variables|Default|GetPlayer))
  (bind _returnvalue_4 (Transformation|GetActorLocation _player))
  (bind _returnvalue_5 (+ _returnvalue (.x _returnvalue_3)))
  (bind _returnvalue_6 (+ _returnvalue_2 (.y _returnvalue_3)))
  (bind _returnvalue_7 (Math|Vector|MakeVector _returnvalue_5 _returnvalue_6 (.z _returnvalue_3)))
  (if (<= (Variables|Default|GetSpawnedTargets) 3)
    (bind _returnvalue_8 (Game|SpawnActorfromClass "/Game/Blueprints/Target.Target_C" (Math|Transform|MakeTransform _returnvalue_7 (Math|Rotator|FindLookatRotation _returnvalue_7 (Math|Vector|MakeVector (.x _returnvalue_4) (.y _returnvalue_4) (.z _returnvalue_3))) "1.000000,1.000000,1.000000") "Undefined" 0 0))
    (Default|SetSpawner _returnvalue_8 self)
    (Math|Integer|IncrementInt (Variables|Default|GetSpawnedTargets))))

(event EventBeginPlay
  (Variables|Default|SetPlayer (Game|Player|GetPlayerPawn 0))
  (Utilities|Time|SetTimerbyEvent (delegate Custom|SpawnTarget) 2.0 true))

(fn ConstructionScript)

(fn HitTarget
  (bind _result (Math|Integer|IncrementInt (Variables|Default|GetHitTargets))
    (:%20%20
      (Default|SetScore (Variables|Default|GetScoreBoard) _result))))