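; Elevator platform actor that rises while the player stands in its trigger box and descends when the player leaves.
; Box overlap begin and end events, filtered to BP_Player, toggle an IsMovingUp flag.
; Tick integrates a clamped height offset at constant speed in the flagged direction and applies it to the Z of the start location captured on BeginPlay.
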(event OnComponentBeginOverlap(Box)
  (params (OverlappedComponent :type Primitive%20Component%20Object%20Reference) (OtherActor :type Actor%20Object%20Reference) (OtherComp :type Primitive%20Component%20Object%20Reference) (OtherBodyIndex :type Integer) (bFromSweep :type Boolean) (SweepResult :type Hit%20Result%20Structure%20%28by%20ref%29))
  (Utilities|Casting|CastToBP_Player OtherActor)
  (Variables|Default|SetisMovingUp true))

(event OnComponentEndOverlap(Box)
  (params (OverlappedComponent :type Primitive%20Component%20Object%20Reference) (OtherActor :type Actor%20Object%20Reference) (OtherComp :type Primitive%20Component%20Object%20Reference) (OtherBodyIndex :type Integer))
  (Utilities|Casting|CastToBP_Player OtherActor)
  (Variables|Default|SetisMovingUp false))

(event EventTick
  (params (DeltaSeconds :type Float%20%28single-precision%29))
  (bind _startlocation (Variables|Default|GetStartLocation))
  (Variables|Default|SetcurrentHeight (Math|Float|Clamp(Float) (+ (Variables|Default|GetcurrentHeight) (* DeltaSeconds (Math|Float|SelectFloat 1e+02 -1e+02 (Variables|Default|GetisMovingUp)))) 0.0 7e+02))
  (Transformation|SetActorLocation (Math|Vector|MakeVector (.x _startlocation) (.y _startlocation) (+ (.z _startlocation) (Variables|Default|GetcurrentHeight))) false false))

(event EventBeginPlay
  (Variables|Default|SetStartLocation (Transformation|GetActorLocation)))

(fn ConstructionScript)