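; Player character Blueprint with walking, sprinting, jumping and a toggle between first-person and third-person cameras.
; Movement follows control yaw in first person and camera boom yaw in third, where the mesh turns to the boom while walking.
; Mouse input, clamped by a sensitivity range, drives the controller or rotates the boom with limited pitch.
; Walk, run and jump flags feed the PlayerAnimator AnimBP, with Tick clearing jump on the ground.
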(event EventBeginPlay
  ;[1 1 1] BeginPlay
  (Utilities|FlowControl|Sequence
    (:then_0
      (bind _asplayer_animator (Utilities|Casting|CastToPlayerAnimator (Components|SkeletalMesh|GetAnimInstance (Variables|Character|GetMesh))))
      (Variables|Default|SetAnimationBP _asplayer_animator))
    (:then_1
      (Components|Activation|Deactivate (Variables|Default|GetCamera)))))

(event EventTick
  (params (DeltaSeconds :type Float%20%28single-precision%29))
  ;[1 1 1] Tick
  (if (AI|Components|NavMovement|IsMovingonGround (Variables|Character|GetCharacterMovement))
    (Variables|/Game/Blueprints/AnimationBlueprints/PlayerAnimator.PlayerAnimator_C|SetisJumping (Variables|Default|GetAnimationBP) false)))

(event Input|ActionEvents|InputActionJump
  (params (Key :type Key%20Structure :default "None"))
  ;[1 1 1] Jumping
  (:Pressed
    (if (AI|Components|NavMovement|IsMovingonGround (Variables|Character|GetCharacterMovement))
      (Character|Jump)
      (Variables|/Game/Blueprints/AnimationBlueprints/PlayerAnimator.PlayerAnimator_C|SetisJumping (Variables|Default|GetAnimationBP) true))))

(event Input|ActionEvents|InputActionSprint
  (params (Key :type Key%20Structure :default "None"))
  (bind _animationbp (Variables|Default|GetAnimationBP))
  (bind _charactermovement (Variables|Character|GetCharacterMovement))
  ;[1 1 1] Sprint
  (:Pressed
    (Variables|/Script/Engine.CharacterMovementComponent|SetMaxWalkSpeed _charactermovement 7e+02)
    (Variables|/Game/Blueprints/AnimationBlueprints/PlayerAnimator.PlayerAnimator_C|SetisRunning _animationbp true))
  (:Released
    (Variables|/Script/Engine.CharacterMovementComponent|SetMaxWalkSpeed _charactermovement 3e+02)
    (Variables|/Game/Blueprints/AnimationBlueprints/PlayerAnimator.PlayerAnimator_C|SetisRunning _animationbp false)))

(event Input|ActionEvents|InputActionChangeView
  (params (Key :type Key%20Structure :default "None"))
  ;[1 1 1] Change View
  (:Pressed
    (Utilities|FlowControl|FlipFlop
      (:A
        (Components|Activation|Deactivate (Variables|Default|GetThirdPersonCamera))
        (Components|Activation|Activate (Variables|Default|GetCamera) false)
        (Variables|Default|SetisFirstPerson true)
        (Transformation|SetRelativeRotation (Variables|Character|GetMesh) "0,-90.000000, 0" false false))
      (:B
        (Components|Activation|Deactivate (Variables|Default|GetCamera))
        (Components|Activation|Activate (Variables|Default|GetThirdPersonCamera) false)
        (Variables|Default|SetisFirstPerson false)
        (Transformation|SetRelativeRotation (Variables|Default|GetCameraBoom) "0, 0, 0" false false)))))

(event Input|AxisEvents|InputAxisHorizontal
  (params (AxisValue :type Float%20%28single-precision%29))
  ;[1 1 1] Movement
  (Pawn|Input|AddMovementInput (Math|Vector|GetRightVector (Math|Rotator|MakeRotator 0.0 0.0 (Math|Float|SelectFloat (.yaw (Pawn|GetControlRotation :!class /Script/Engine.Pawn)) (.yaw (Transformation|GetWorldRotation (Variables|Default|GetCameraBoom))) (Variables|Default|GetisFirstPerson)))) AxisValue false)
  (bind _output_get (Variables|/Game/Blueprints/AnimationBlueprints/PlayerAnimator.PlayerAnimator_C|SetisWalking (Variables|Default|GetAnimationBP) (> (Math|Float|Absolute(Float) (+ AxisValue (stale Input|AxisEvents|InputAxisVertical AxisValue))) 0.0)))
  (if (and (not (Variables|Default|GetisFirstPerson)) _output_get)
    (Transformation|SetRelativeRotation (Variables|Character|GetMesh) (Math|Rotator|MakeRotator 0.0 0.0 (- (.yaw (Variables|/Script/Engine.SceneComponent|GetRelativeRotation (Variables|Default|GetCameraBoom))) 9e+01)) false false)))

(event Input|AxisEvents|InputAxisVertical
  (params (AxisValue :type Float%20%28single-precision%29))
  ;[1 1 1] Movement
  (Pawn|Input|AddMovementInput (Math|Vector|GetForwardVector (Math|Rotator|MakeRotator 0.0 0.0 (Math|Float|SelectFloat (.yaw (Pawn|GetControlRotation :!class /Script/Engine.Pawn)) (.yaw (Transformation|GetWorldRotation (Variables|Default|GetCameraBoom))) (Variables|Default|GetisFirstPerson)))) AxisValue false)
  (bind _output_get (Variables|/Game/Blueprints/AnimationBlueprints/PlayerAnimator.PlayerAnimator_C|SetisWalking (Variables|Default|GetAnimationBP) (> (Math|Float|Absolute(Float) (+ (stale Input|AxisEvents|InputAxisHorizontal AxisValue) AxisValue)) 0.0)))
  (if (and (not (Variables|Default|GetisFirstPerson)) _output_get)
    (Transformation|SetRelativeRotation (Variables|Character|GetMesh) (Math|Rotator|MakeRotator 0.0 0.0 (- (.yaw (Variables|/Script/Engine.SceneComponent|GetRelativeRotation (Variables|Default|GetCameraBoom))) 9e+01)) false false)))

(event Input|AxisEvents|InputAxisMouseY
  (params (AxisValue :type Float%20%28single-precision%29))
  (bind _minmaxsensitivity (Variables|Default|GetMinMaxSensitivity))
  (bind _cameraboom (Variables|Default|GetCameraBoom))
  (bind _isfirstperson (Variables|Default|GetisFirstPerson))
  (bind _invertmousethirdperson (Variables|Default|GetInvertMouseThirdPerson))
  (bind _returnvalue (Math|Float|SelectFloat 1.0 -1.0 _invertmousethirdperson))
  (bind _relativerotation (Variables|/Script/Engine.SceneComponent|GetRelativeRotation _cameraboom))
  (bind _returnvalue_2 (Math|Float|SelectFloat 1.0 _returnvalue _isfirstperson))
  (bind _returnvalue_3 (* AxisValue _returnvalue_2))
  (bind _returnvalue_4 (Math|Float|Clamp(Float) _returnvalue_3 (.x _minmaxsensitivity) (.y _minmaxsensitivity)))
  ;[1 1 1] Look Around
  (if (Variables|Default|GetisFirstPerson)
    (Pawn|Input|AddControllerPitchInput _returnvalue_4)
    (else
      (Transformation|SetRelativeRotation (Variables|Default|GetCameraBoom) (Math|Rotator|MakeRotator (.roll _relativerotation) (Math|Float|Clamp(Float) (+ _returnvalue_4 (.pitch _relativerotation)) -7e+01 7e+01) (.yaw _relativerotation)) false false))))

(event Input|AxisEvents|InputAxisMouseX
  (params (AxisValue :type Float%20%28single-precision%29))
  (bind _minmaxsensitivity (Variables|Default|GetMinMaxSensitivity))
  (bind _returnvalue (Math|Float|Clamp(Float) AxisValue (.x _minmaxsensitivity) (.y _minmaxsensitivity)))
  ;[1 1 1] Look Around
  (if (Variables|Default|GetisFirstPerson)
    (Pawn|Input|AddControllerYawInput _returnvalue)
    (else
      (Transformation|AddRelativeRotation (Variables|Default|GetCameraBoom) (Math|Rotator|MakeRotator 0.0 0.0 _returnvalue) false false))))

(fn ConstructionScript)