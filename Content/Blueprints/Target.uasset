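; Target actor that arrows destroy on contact, reporting hits to the spawner that manages it.
; A spawner reference is handed in through SetSpawner.
; When an Arrow overlaps the static mesh, it calls HitTarget on the spawner, then destroys both the arrow and itself.
; On destruction it decrements the spawner's count of spawned targets.
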(event OnComponentBeginOverlap(StaticMesh)
  (params (OverlappedComponent :type Primitive%20Component%20Object%20Reference) (OtherActor :type Actor%20Object%20Reference) (OtherComp :type Primitive%20Component%20Object%20Reference) (OtherBodyIndex :type Integer) (bFromSweep :type Boolean) (SweepResult :type Hit%20Result%20Structure%20%28by%20ref%29))
  (bind _asarrow (Utilities|Casting|CastToArrow OtherActor))
  (Default|HitTarget (Variables|Default|GetSpawner))
  (Actor|DestroyActor _asarrow)
  (Actor|DestroyActor))

(event Custom|SetSpawner
  (params (Spawner :type Target%20Spawner%20Object%20Reference))
  (Variables|Default|SetSpawner Spawner))

(event EventDestroyed
  (Math|Integer|DecrementInt (Variables|/Game/Blueprints/TargetSpawner.TargetSpawner_C|GetSpawnedTargets (Variables|Default|GetSpawner))))

(fn ConstructionScript)