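; Actor that continuously slides back and forth along world Y between the MinMax offsets from its BeginPlay location.
; Tick flips the IsMovingUp direction flag at either limit, then applies Speed scaled by delta time, clamps the offset and sets the actor location.
; BP_Player entering the Box forces movement toward positive Y, and leaving it forces movement toward negative Y.
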(event OnComponentBeginOverlap(Box)
  (params (OverlappedComponent :type Primitive%20Component%20Object%20Reference) (OtherActor :type Actor%20Object%20Reference) (OtherComp :type Primitive%20Component%20Object%20Reference) (OtherBodyIndex :type Integer) (bFromSweep :type Boolean) (SweepResult :type Hit%20Result%20Structure%20%28by%20ref%29))
  (Utilities|Casting|CastToBP_Player OtherActor)
  (Variables|Default|SetisMovingUp true))

(event OnComponentEndOverlap(Box)
  (params (OverlappedComponent :type Primitive%20Component%20Object%20Reference) (OtherActor :type Actor%20Object%20Reference) (OtherComp :type Primitive%20Component%20Object%20Reference) (OtherBodyIndex :type Integer))
  (Utilities|Casting|CastToBP_Player OtherActor)
  (Variables|Default|SetisMovingUp false))

(event EventTick
  (params (DeltaSeconds :type Float%20%28single-precision%29))
  (bind _minmax (Variables|Default|GetminMax))
  (bind _speed (Variables|Default|Getspeed))
  (bind _startlocation (Variables|Default|GetStartLocation))
  (bind _minmax_2 (Variables|Default|GetminMax))
  (Utilities|FlowControl|Sequence
    (:then_0
      (if (or (and (Variables|Default|GetisMovingUp) (>= (Variables|Default|GetcurrentY) (.y _minmax_2))) (and (not (Variables|Default|GetisMovingUp)) (<= (Variables|Default|GetcurrentY) (.x _minmax_2))))
        (Variables|Default|SetisMovingUp (not (Variables|Default|GetisMovingUp)))))
    (:then_1
      (Variables|Default|SetcurrentY (Math|Float|Clamp(Float) (+ (Variables|Default|GetcurrentY) (* DeltaSeconds (Math|Float|SelectFloat _speed (* _speed -1.0) (Variables|Default|GetisMovingUp)))) (.x _minmax) (.y _minmax)))
      (Transformation|SetActorLocation (Math|Vector|MakeVector (.x _startlocation) (+ (.y _startlocation) (Variables|Default|GetcurrentY)) (.z _startlocation)) false false))))

(event EventBeginPlay
  (Variables|Default|SetStartLocation (Transformation|GetActorLocation)))

(fn ConstructionScript)