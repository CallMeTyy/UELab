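; BP_ScoreBoard is an actor that shows a score through a widget.
; Its SetScore function casts the Widget component's user widget to ScoreBoard and sets the ScoreText to the integer score.
; If the cast fails, nothing is updated.
; The event graph and construction script add no logic of their own.
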(event EventBeginPlay
  (|CallParentFunction) ; This node is disabled and will not be called.\nDrag off pins to build functionality.
)

(event Collision|EventActorBeginOverlap
  (params (OtherActor :type Actor%20Object%20Reference))
  (|CallParentFunction OtherActor) ; This node is disabled and will not be called.\nDrag off pins to build functionality.
)

(event EventTick
  (params (DeltaSeconds :type Float%20%28single-precision%29))
  (|CallParentFunction DeltaSeconds) ; This node is disabled and will not be called.\nDrag off pins to build functionality.
)

(fn ConstructionScript
  (|CallParentFunction))

(fn SetScore
  (params (Score :type Integer))
  (bind _asscore_board (Utilities|Casting|CastToScoreBoard (UserInterface|GetWidget (Variables|Default|GetWidget))))
  (Rendering|Components|TextRender|SetText (Variables|/Game/Blueprints/WidgetBlueprints/ScoreBoard.ScoreBoard_C|GetScoreText _asscore_board) (Utilities|Text|ToText(Integer) Score)))